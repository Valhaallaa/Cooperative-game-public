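; Interactable crank actor that turns another actor when used.
; WhenInteracted adds a Rotationamount yaw step in local space to both the referenced Rotationactor and its own Cube1 component, then plays a 2D lever sound.
; Disconnected leftover nodes hold an older CrankValue-threshold rotation and an ordered-sequence check, neither of which runs.
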(event `self.WhenInteracted`
  (bind _returnvalue (`KismetMathLibrary.MakeRotator` 0.0 0.0 (`self.rotationamount`)))
  (`self.K2_AddActorLocalRotation` (`self.rotationactor`) _returnvalue false false)
  (`SceneComponent.K2_AddLocalRotation` (`self.Cube1`) _returnvalue false false)
  (`GameplayStatics.PlaySound2D` "/Game/Audio/GameAudio/FoleyAudio/Lever.Lever" 1.0 1.0 0.0 null null))

(event `self.ReceiveTick`
  (params (DeltaSeconds :type "Float (single-precision)")))

(fn `UserConstructionScript`)