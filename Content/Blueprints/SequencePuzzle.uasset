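; Trigger actor that shows the sequence puzzle UI while a character stands in its volume.
; On overlap it finds a BP_SequencePuzzle via GetActorOfClass and, if that puzzle is not complete, creates a Sequence_puzzle widget for player 0.
; Leaving the trigger calls RemoveAllWidgets, clearing every widget on screen rather than only the puzzle's.
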(event `self.Trigger.OnComponentBeginOverlap`
  (params (OverlappedComponent :type "PrimitiveComponent Object Reference") (OtherActor :type "Actor Object Reference") (OtherComp :type "PrimitiveComponent Object Reference") (OtherBodyIndex :type Integer) (bFromSweep :type Boolean) (SweepResult :type "HitResult Structure (by ref)"))
  (cast `Character` OtherActor)
  (bind _returnvalue (`GameplayStatics.GetActorOfClass` "/Game/Blueprints/BP_SequencePuzzle.BP_SequencePuzzle_C"))
  (bind _asbp_sequence_puzzle (cast `/Game/Blueprints/BP_SequencePuzzle` _returnvalue))
  (if (not (`/Game/Blueprints/BP_SequencePuzzle.isComplete` _asbp_sequence_puzzle))
    (bind _returnvalue_2 (`|CreateWidget` "/Game/UI/3Dview/Widgets/Sequence_puzzle.Sequence_puzzle_C" (`GameplayStatics.GetPlayerController` 0)))
    (`UserWidget.AddToViewport` _returnvalue_2 0)))

(event `self.Trigger.OnComponentEndOverlap`
  (params (OverlappedComponent :type "PrimitiveComponent Object Reference") (OtherActor :type "Actor Object Reference") (OtherComp :type "PrimitiveComponent Object Reference") (OtherBodyIndex :type Integer))
  (cast `Character` OtherActor)
  (`WidgetLayoutLibrary.RemoveAllWidgets`))

(fn `UserConstructionScript`)