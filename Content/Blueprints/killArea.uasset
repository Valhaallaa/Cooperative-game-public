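; Kill zone actor that sends either of two player characters back to a respawn point on contact.
; When its Cube is overlapped, it casts the actor to tell BP_ThirdPersonCharacter (player 1) from BP_ThirdPersonCharacter2 (player 0).
; It then gets that player's character and respawn location from BP_Gamemode, moving the looked-up character there rather than the overlapping actor reference.
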(event `self.Cube.OnComponentBeginOverlap`
  (params (OverlappedComponent :type "PrimitiveComponent Object Reference") (OtherActor :type "Actor Object Reference") (OtherComp :type "PrimitiveComponent Object Reference") (OtherBodyIndex :type Integer) (bFromSweep :type Boolean) (SweepResult :type "HitResult Structure (by ref)"))
  (bind _returnvalue (`GameplayStatics.GetGameMode`))
  (cast `/Game/Blueprints/BP_ThirdPersonCharacter` OtherActor
    (:`then`
      (bind _asbp_gamemode (cast `/Game/Blueprints/BP_Gamemode` _returnvalue))
      (bind _returnvalue_2 (`MyProjectGameMode.GetP1Respawn` _asbp_gamemode))
      (bind _returnvalue_3 (`MyProjectGameMode.GetCharacter` _asbp_gamemode 1))
      (`self.K2_SetActorLocation` _returnvalue_3 _returnvalue_2 false false))
    (:`CastFailed`
      (cast `/Game/Blueprints/BP_ThirdPersonCharacter2` OtherActor)
      (bind _asbp_gamemode_2 (cast `/Game/Blueprints/BP_Gamemode` _returnvalue))
      (bind _returnvalue_4 (`MyProjectGameMode.GetP0Respawn` _asbp_gamemode_2))
      (bind _returnvalue_5 (`MyProjectGameMode.GetCharacter` _asbp_gamemode_2 0))
      (`self.K2_SetActorLocation` _returnvalue_5 _returnvalue_4 false false))))

(fn `UserConstructionScript`)