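; Interactable crank that raises a referenced actor one step per use, then lets it sink back after three seconds without use.
; Each interaction lifts Rotationactor up to Max, spins Cube1, plays a lever sound and resets the countdown here and on an optional linked crank.
; Tick then lowers it by a fifth of a step per frame, independent of frame time, down to its BeginPlay height, spinning Cube1 backwards.
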(event `self.ReceiveTick`
  (params (DeltaSeconds :type "Float (single-precision)"))
  (bind _rotationactor (`self.rotationactor`))
  (bind (_returnvalue_x _returnvalue_y _returnvalue_z) (`KismetMathLibrary.BreakVector` (`self.K2_GetActorLocation` _rotationactor)))
  (bind _returnvalue (- _returnvalue_z (/ (`self.raiseAmount`) 5.0)))
  (bind _output_get (set `self.Decrease time` (- (`self.Decrease time`) DeltaSeconds)))
  (if (<= _output_get 0.0)
    (if (>= _returnvalue (`self.Min`))
      (`self.K2_SetActorLocation` _rotationactor (`KismetMathLibrary.MakeVector` _returnvalue_x _returnvalue_y _returnvalue) false false)
      (`SceneComponent.K2_AddLocalRotation` (`self.Cube1`) (`KismetMathLibrary.MakeRotator` 0.0 0.0 (* (`self.raiseAmount`) -1.0)) false false))))

(event `self.ReceiveBeginPlay`
  (bind (_returnvalue_x _returnvalue_y _returnvalue_z) (`KismetMathLibrary.BreakVector` (`self.K2_GetActorLocation` (`self.rotationactor`))))
  (set `self.Min` _returnvalue_z))

(event `self.WhenInteracted`
  (bind _crank (`self.Crank`))
  (bind _rotationactor (`self.rotationactor`))
  (bind (_returnvalue_x _returnvalue_y _returnvalue_z) (`KismetMathLibrary.BreakVector` (`self.K2_GetActorLocation` _rotationactor)))
  (bind _returnvalue (+ _returnvalue_z (`self.raiseAmount`)))
  (if (<= _returnvalue (`self.Max`))
    (`self.K2_SetActorLocation` _rotationactor (`KismetMathLibrary.MakeVector` _returnvalue_x _returnvalue_y _returnvalue) false false)
    (`GameplayStatics.PlaySound2D` "/Game/Audio/GameAudio/FoleyAudio/Lever.Lever" 1.0 1.0 0.0 null null)
    (set `self.Decrease time` 3.0)
    (`SceneComponent.K2_AddLocalRotation` (`self.Cube1`) (`KismetMathLibrary.MakeRotator` 0.0 0.0 (`self.raiseAmount`)) false false)
    (if (`KismetSystemLibrary.IsValid` _crank)
      (bind _asbp_crank_raise (cast `/Game/Blueprints/BP_CrankRaise` _crank))
      (set `/Game/Blueprints/BP_CrankRaise.Decrease time` 3.0 _asbp_crank_raise))))

(fn `UserConstructionScript`)