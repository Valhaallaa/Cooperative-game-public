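; BP_LightPP is a pressure plate that activates while tagged actors step on it and deactivates when they leave.
; Overlap events on Cube1 check the other actor against the TagsActivate list, then call ActivateLoop or DeActivateLoop, neither defined here.
; Cube's material switches between glowing and non-glowing to show the state.
; Overlaps are not counted, so any matching actor leaving deactivates the plate.
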(event `self.Cube1.OnComponentBeginOverlap`
  (params (OverlappedComponent :type "PrimitiveComponent Object Reference") (OtherActor :type "Actor Object Reference") (OtherComp :type "PrimitiveComponent Object Reference") (OtherBodyIndex :type Integer) (bFromSweep :type Boolean) (SweepResult :type "HitResult Structure (by ref)"))
  (for _array_element (`self.TagsActivate`)
    (if (`self.ActorHasTag` OtherActor _array_element)
      (`self.ActivateLoop`)
      (`PrimitiveComponent.SetMaterial` (`self.Cube`) 0 "/Game/Assets/PreasurePlate/PreasurePlate_Material.PreasurePlate_Material"))))

(event `self.Cube1.OnComponentEndOverlap`
  (params (OverlappedComponent :type "PrimitiveComponent Object Reference") (OtherActor :type "Actor Object Reference") (OtherComp :type "PrimitiveComponent Object Reference") (OtherBodyIndex :type Integer))
  (for _array_element (`self.TagsActivate`)
    (if (`self.ActorHasTag` OtherActor _array_element)
      (`self.DeActivateLoop`)
      (`PrimitiveComponent.SetMaterial` (`self.Cube`) 0 "/Game/Assets/PreasurePlate/PreasurePlate_NoneGlow.PreasurePlate_NoneGlow"))))

(fn `UserConstructionScript`)