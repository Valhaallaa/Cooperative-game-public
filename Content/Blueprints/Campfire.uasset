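; Campfire trigger that moves a two-character game to another level once both characters gather in it.
; Overlap events track actors in CurrentChars, whose first two entries are matched against the first instances of the two third-person character classes.
; When both match, it fades the camera and audio out, removes the second local player if present, then opens the level named by SceneNane.
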(event `self.trigger.OnComponentBeginOverlap`
  (params (OverlappedComponent :type "PrimitiveComponent Object Reference") (OtherActor :type "Actor Object Reference") (OtherComp :type "PrimitiveComponent Object Reference") (OtherBodyIndex :type Integer) (bFromSweep :type Boolean) (SweepResult :type "HitResult Structure (by ref)"))
  (bind _returnvalue (`GameplayStatics.GetPlayerController` 1))
  (bind _currentchars (`self.CurrentChars`))
  (bind _output (`|GetArrayItem` _currentchars))
  (bind _output_2 (`|GetArrayItem` _currentchars 1))
  (`KismetArrayLibrary.Array_Add` _currentchars OtherActor)
  (bind _outactors (`GameplayStatics.GetAllActorsOfClass` "/Game/Blueprints/BP_ThirdPersonCharacter.BP_ThirdPersonCharacter_C"))
  (bind _outactors_2 (`GameplayStatics.GetAllActorsOfClass` "/Game/Blueprints/BP_ThirdPersonCharacter2.BP_ThirdPersonCharacter2_C"))
  (bind _outactors_3 (`GameplayStatics.GetAllActorsOfClass` "/Game/Blueprints/BP_ThirdPersonCharacter2.BP_ThirdPersonCharacter2_C"))
  (bind _outactors_4 (`GameplayStatics.GetAllActorsOfClass` "/Game/Blueprints/BP_ThirdPersonCharacter.BP_ThirdPersonCharacter_C"))
  (set `self.car 1 here` (or (== _output (`|GetArrayItem` _outactors)) (== _output (`|GetArrayItem` _outactors_2))))
  (set `self.car 2 here` (or (== _output_2 (`|GetArrayItem` _outactors_4)) (== _output_2 (`|GetArrayItem` _outactors_3))))
  (if (and (`self.car 1 here`) (`self.car 2 here`))
    (cast `Character` OtherActor)
    (`PlayerCameraManager.StartCameraFade` :`self` (`GameplayStatics.GetPlayerCameraManager` 0) :`ToAlpha` 1.0 :`Duration` 2.0 :`bShouldFadeAudio` true :`bHoldWhenFinished` true)
    (`KismetSystemLibrary.Delay` 2.0)
    (if (`KismetSystemLibrary.IsValid` _returnvalue)
      (`GameplayStatics.RemovePlayer` _returnvalue))
    (`GameplayStatics.OpenLevel` (`self.SceneNane`))))

(event `self.trigger.OnComponentEndOverlap`
  (params (OverlappedComponent :type "PrimitiveComponent Object Reference") (OtherActor :type "Actor Object Reference") (OtherComp :type "PrimitiveComponent Object Reference") (OtherBodyIndex :type Integer))
  (`KismetArrayLibrary.Array_RemoveItem` (`self.CurrentChars`) OtherActor))

(fn `UserConstructionScript`)