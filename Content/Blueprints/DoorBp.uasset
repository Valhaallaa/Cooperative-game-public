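; DoorBp is a double door that opens when a BP_ThirdPersonCharacter overlaps its Trigger, then loads another level.
; The OpenDoor timeline sets the yaw of Point1 and Point2 from separate angle tracks.
; Each timeline update also calls a three-second camera fade starting at full alpha and reaches a three-second Delay that leads to opening LevelName.
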(event `self.Trigger.OnComponentBeginOverlap`
  (params (OverlappedComponent :type "PrimitiveComponent Object Reference") (OtherActor :type "Actor Object Reference") (OtherComp :type "PrimitiveComponent Object Reference") (OtherBodyIndex :type Integer) (bFromSweep :type Boolean) (SweepResult :type "HitResult Structure (by ref)"))
  (cast `/Game/Blueprints/BP_ThirdPersonCharacter` OtherActor)
  (`Timeline|Open Door`
    (:`Update`
      (`SceneComponent.K2_SetRelativeRotation` (`self.Point1`) (`KismetMathLibrary.MakeRotator` 0.0 0.0 (`self.Door_1_OpenAngle`)) false false)
      (`SceneComponent.K2_SetRelativeRotation` (`self.Point2`) (`KismetMathLibrary.MakeRotator` 0.0 0.0 (`self.Door_2_OpenAngle`)) false false)
      (`PlayerCameraManager.StartCameraFade` :`self` (`GameplayStatics.GetPlayerCameraManager` 0) :`FromAlpha` 1.0 :`Duration` 3.0)
      (`KismetSystemLibrary.Delay` 3.0)
      (`GameplayStatics.OpenLevel` (`self.Level Name`)))))

(fn `UserConstructionScript`)