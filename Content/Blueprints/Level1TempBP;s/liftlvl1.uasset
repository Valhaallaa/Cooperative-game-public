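; Level 1 lift actor that raises or lowers its Lift component according to a rotation value passed to MoveLift.
; Each call eases the lift to a height scaled from that rotation, feeding its world X and Y in as the relative target.
; A retriggerable delay follows; if Reset is set, it clears Reset on the first Cranklvl1 found and eases the lift to relative zero.
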(event `MoveLift`
  (params (CurrentRotation :type "Float (double-precision)") (reset :type Boolean))
  (bind (_returnvalue_x _returnvalue_y) (`KismetMathLibrary.BreakVector` (`SceneComponent.K2_GetComponentLocation` (`self.Lift`))))
  (`|ExecutionSequence`
    (:`then_0`
      (`KismetSystemLibrary.RetriggerableDelay` 3.0)
      (if reset
        (bind _outactors (`GameplayStatics.GetAllActorsOfClass` "/Game/Blueprints/Level1TempBP;s/cranklvl1.cranklvl1_C"))
        (set `/Game/Blueprints/Level1TempBP;s/cranklvl1.reset` false (`|GetArrayItem` _outactors))
        (`KismetSystemLibrary.MoveComponentTo` (`self.Lift`) (0.0 0.0 0.0) (struct) false false 1.0)))
    (:`then_1`
      (`KismetSystemLibrary.MoveComponentTo` (`self.Lift`) (`KismetMathLibrary.MakeVector` _returnvalue_x _returnvalue_y (+ (* CurrentRotation 2.5) 54.0)) (struct) false false 1.0))))

(fn `UserConstructionScript`)