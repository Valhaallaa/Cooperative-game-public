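; RisingBridge is a bridge actor whose Cube component rises when the required number of interacts are active.
; BeginPlay stores a lowered or offset rest position from StartSinkAmount and moves the cube at start.
; OnActivate raises it by RaiseAmount when InteractsActive equals InteractsNeeded, and StopActivate returns it to rest when the count falls short.
; Movement uses timed MoveComponentTo, while Tick keeps the active count from going negative.
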(event `self.ReceiveBeginPlay`
  (set `self.oldHeight` (`KismetMathLibrary.MakeVector` (.x (`SceneComponent.RelativeLocation` (`self.Cube`))) (.y (`SceneComponent.RelativeLocation` (`self.Cube`))) (+ (.z (`SceneComponent.RelativeLocation` (`self.Cube`))) (`self.StartSinkAmount`))))
  (`/Engine/EditorBlueprintResources/StandardMacros.DoOnce` false
    (:`Completed`
      (`KismetSystemLibrary.MoveComponentTo` (`self.Cube`) (`KismetMathLibrary.MakeVector` 0.0 0.0 (`self.StartSinkAmount`)) (struct) false false 1.0))))

(event `self.ReceiveTick`
  (params (DeltaSeconds :type "Float (single-precision)"))
  (if (< (`self.interactsActive`) 0)
    (set `self.interactsActive` 0)))

(event `self.OnActivate`
  (if (== (`self.interactsNeeded`) (`self.interactsActive`))
    (`KismetSystemLibrary.PrintString` "true")
    (`KismetMathLibrary.Vector_Set` (`self.newHeight`) (.x (`self.oldHeight`)) (.y (`self.oldHeight`)) (+ (.z (`self.oldHeight`)) (`self.RaiseAmount`)))
    (`KismetSystemLibrary.MoveComponentTo` (`self.Cube`) (`self.newHeight`) (struct) false false 1.0)
    (set `self.isActivated` true)
    (else
      (`KismetSystemLibrary.PrintString` "fakse"))))

(event `self.StopActivate`
  (if (> (`self.interactsNeeded`) (`self.interactsActive`))
    (`KismetSystemLibrary.MoveComponentTo` (`self.Cube`) (`self.oldHeight`) (struct) false false 1.0)
    (set `self.isActivated` false)))

(fn `UserConstructionScript`)