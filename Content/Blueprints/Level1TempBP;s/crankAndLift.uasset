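; Crank-and-lift actor that lets the player raise a lift by pressing Interact while inside a box trigger, which toggles input.
; Each press steps the crank's rotation by 36 degrees until it reaches a full turn, and moves the lift to a height proportional to that rotation.
; When presses stop, retriggerable delays and a looping wire step the crank back down, lowering the lift and resetting the first-press state.
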(event `self.Box.OnComponentBeginOverlap`
  (params (OverlappedComponent :type "PrimitiveComponent Object Reference") (OtherActor :type "Actor Object Reference") (OtherComp :type "PrimitiveComponent Object Reference") (OtherBodyIndex :type Integer) (bFromSweep :type Boolean) (SweepResult :type "HitResult Structure (by ref)"))
  (`self.EnableInput` (`GameplayStatics.GetPlayerController` 0)))

(event `self.Box.OnComponentEndOverlap`
  (params (OverlappedComponent :type "PrimitiveComponent Object Reference") (OtherActor :type "Actor Object Reference") (OtherComp :type "PrimitiveComponent Object Reference") (OtherBodyIndex :type Integer))
  (`self.DisableInput` (`GameplayStatics.GetPlayerController` 0)))

(event `InputAction|Interact`
  (params (Key :type "Key Structure"))
  (bind _current_rotation (`self.Current Rotation`))
  (bind _current_rotation_2 (`self.Current Rotation`))
  (:`Pressed`
    (`KismetSystemLibrary.Delay` 0.5)
    (if (`self.firstpass`)
      (`SceneComponent.K2_SetRelativeRotation` (`self.Crank2`) (`KismetMathLibrary.MakeRotator` -90.0 36.0) false false)
      (set `self.firstpass` false)
      (`KismetSystemLibrary.Delay` 2.0)
      (if (not (`self.isRotating`))
        (`SceneComponent.K2_SetRelativeRotation` (`self.Crank2`) (`KismetMathLibrary.MakeRotator` -90.0) false false))
      (else
        (`KismetSystemLibrary.PrintString` (`KismetStringLibrary.Conv_DoubleToString` (`self.Current Rotation`)))
        (if (not (== (`self.Current Rotation`) 360.0))
          (set `self.isRotating` true)
          (`|ExecutionSequence`
            (:`then_0`
              (`KismetSystemLibrary.RetriggerableDelay` 2.0)
              (set `self.isRotating` false))
            (:`then_1`
              ;[1 1 1] Value going up
              (`SceneComponent.K2_SetRelativeRotation` (`self.Crank2`) (`KismetMathLibrary.MakeRotator` -90.0 _current_rotation) false false)
              (set `self.Current Rotation` (+ _current_rotation 36.0))
              ;[1 1 1] Value going Down
              (if (== (`self.Current Rotation`) 36.0) :!label _label
                (set `self.firstpass` true)
                (set `self.Current Rotation` 36.0)
                (set `self.reset` true)
                (else
                  (`KismetSystemLibrary.Delay` 2.0 :!label _label_2)
                  (if (`self.isRotating`)
                    (goto _label_2)
                    (else
                      (`|ExecutionSequence`
                        (:`then_0`
                          (`SceneComponent.K2_SetRelativeRotation` (`self.Crank2`) (`KismetMathLibrary.MakeRotator` -90.0 (`self.Current Rotation`)) false false)
                          (if (== _current_rotation_2 0.0)
                            (goto _label)
                            (else
                              (set `self.Current Rotation` (+ _current_rotation_2 -36.0))
                              (goto _label))))
                        (:`then_1`
                          (`KismetSystemLibrary.RetriggerableDelay` 3.0)
                          (if (`self.reset`)
                            (set `self.reset` false)
                            (`KismetSystemLibrary.MoveComponentTo` (`self.Lift`) (0.0 0.0 0.0) (struct) false false 2.0)
                            (`SceneComponent.K2_SetRelativeRotation` (`self.Crank2`) (`KismetMathLibrary.MakeRotator` -90.0) false false)))
                        (:`then_2`
                          (`KismetSystemLibrary.MoveComponentTo` (`self.Lift`) (`KismetMathLibrary.MakeVector` 0.0 0.0 (* (`self.Current Rotation`) 2.5)) (struct) false false 2.0 :!label _label_3))))))))))))))

(event `InputAction|Interact`
  (params (Key :type "Key Structure"))
  (:`Pressed`
    (`KismetSystemLibrary.Delay` 0.5)
    (goto _label_3)))

(fn `UserConstructionScript`)