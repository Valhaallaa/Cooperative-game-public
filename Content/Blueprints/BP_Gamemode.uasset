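; Game mode for a game with optional two-player play, handling pausing, player spawning and collectable progress across three levels.
; BeginPlay reads the two-player flag from the game instance, adding a player and loading or creating the save when set.
; Save, Load and Reset sync per-level counts and completion flags with BP_SaveGameInfo, saving asynchronously.
; Tick respawns missing characters, while events toggle the pause menu and gamepad assignment.
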(event `self.PauseGame`
  (bind _returnvalue (`GameplayStatics.GetPlayerController` 0))
  (`KismetSystemLibrary.PrintString` "pause")
  (if (`self.paused`)
    (if (`KismetSystemLibrary.IsValid` (stale _returnvalue_3))
      (`Widget.RemoveFromParent` (stale _returnvalue_3))
      (bind _returnvalue_2 (`GameplayStatics.SetGamePaused` false))
      (set `self.paused` _returnvalue_2)
      (`WidgetBlueprintLibrary.SetInputMode_GameOnly` _returnvalue))
    (else
      (bind _returnvalue_3 (`|CreateWidget` "/Game/UI/3Dview/Widgets/PauseMenu.PauseMenu_C" _returnvalue))
      (`UserWidget.AddToViewport` _returnvalue_3 0)
      (bind _returnvalue_4 (`GameplayStatics.SetGamePaused` true))
      (set `self.paused` _returnvalue_4))))

(event `self.SaveGame`
  (bind _save_game_instance (`self.Save Game Instance`))
  (bind _save_game_instance_2 (`self.Save Game Instance`))
  (`KismetSystemLibrary.PrintString` "Save")
  (`|ExecutionSequence`
    (:`then_0`
      (set `/Game/Blueprints/BP_SaveGameInfo.L1AllCollectablesFound` (`self.L1_CollComplete`) _save_game_instance_2))
    (:`then_1`
      (set `/Game/Blueprints/BP_SaveGameInfo.L2AllCollectablesFound` (`self.L2_CollComplete`) _save_game_instance_2))
    (:`then_2`
      (set `/Game/Blueprints/BP_SaveGameInfo.L3AllCollectablesFound` (`self.L3_CollComplete`) _save_game_instance_2))
    (:`then_3`
      (set `/Game/Blueprints/BP_SaveGameInfo.L1CollectablesFound` (`self.L1_CollectedNum`) _save_game_instance_2))
    (:`then_4`
      (set `/Game/Blueprints/BP_SaveGameInfo.L2CollectablesFound` (`self.L2_CollectedNum`) _save_game_instance_2))
    (:`then_5`
      (set `/Game/Blueprints/BP_SaveGameInfo.L3CollectablesFound` (`self.L3_CollectedNum`) _save_game_instance_2))
    (:`then_6`
      (`AsyncActionHandleSaveGame.AsyncSaveGameToSlot` _save_game_instance (`/Game/Blueprints/BP_SaveGameInfo.SaveSlotName` _save_game_instance) (`/Game/Blueprints/BP_SaveGameInfo.UserIndex` _save_game_instance)))))

(event `self.ReceiveBeginPlay`
  (bind _asbp_game_instance (cast `/Game/Blueprints/BP_GameInstance` (`GameplayStatics.GetGameInstance`)))
  (bind _output_get (set `self.twoPlayer` (`/Game/Blueprints/BP_GameInstance.twoPlayersInst` _asbp_game_instance)))
  (if _output_get
    (`self.AddPlayer`)
    (bind _returnvalue (`GameplayStatics.DoesSaveGameExist` "TestSaveSlot"))
    (if _returnvalue
      (bind _returnvalue_2 (`GameplayStatics.LoadGameFromSlot` "TestSaveSlot"))
      (bind _asbp_save_game_info (cast `/Game/Blueprints/BP_SaveGameInfo` _returnvalue_2))
      (`|ExecutionSequence`
        (:`then_0`
          (set `self.Save Game Instance` _asbp_save_game_info)
          (for _array_element (`/Game/Blueprints/BP_SaveGameInfo.CollectablesFound` _asbp_save_game_info)
            (`self.SetActorHiddenInGame` _array_element true))
          (`KismetSystemLibrary.PrintString` (`KismetStringLibrary.Conv_IntToString` (`/Game/Blueprints/BP_SaveGameInfo.L1CollectablesFound` _asbp_save_game_info))))
        (:`then_1`
          (set `self.L1_CollectedNum` (`/Game/Blueprints/BP_SaveGameInfo.L1CollectablesFound` _asbp_save_game_info)))
        (:`then_2`
          (set `self.L2_CollectedNum` (`/Game/Blueprints/BP_SaveGameInfo.L2CollectablesFound` _asbp_save_game_info)))
        (:`then_3`
          (set `self.L3_CollectedNum` (`/Game/Blueprints/BP_SaveGameInfo.L3CollectablesFound` _asbp_save_game_info)))
        (:`then_4`
          (set `self.L1_CollComplete` (`/Game/Blueprints/BP_SaveGameInfo.L1AllCollectablesFound` _asbp_save_game_info)))
        (:`then_5`
          (set `self.L2_CollComplete` (`/Game/Blueprints/BP_SaveGameInfo.L2AllCollectablesFound` _asbp_save_game_info)))
        (:`then_6`
          (set `self.L3_CollComplete` (`/Game/Blueprints/BP_SaveGameInfo.L3AllCollectablesFound` _asbp_save_game_info))))
      (else
        (bind _returnvalue_3 (`GameplayStatics.CreateSaveGameObject` "/Game/Blueprints/BP_SaveGameInfo.BP_SaveGameInfo_C"))
        (set `self.Save Game Instance` _returnvalue_3)))))

(event `self.ReceiveTick`
  (params (DeltaSeconds :type "Float (single-precision)"))
  (set `PlayerController.bShowMouseCursor` true (`GameplayStatics.GetPlayerController` 0))
  (if (`self.initialAddComplete`)
    (bind _returnvalue (`self.GetCharacter` 0))
    (if (`KismetSystemLibrary.IsValid` _returnvalue)
      (bind _returnvalue_2 (`self.GetCharacter` 1))
      (if (not (`KismetSystemLibrary.IsValid` _returnvalue_2))
        (bind _returnvalue_3 (`self.GetP1Respawn`))
        (`|SpawnActorFromClass` "/Game/Blueprints/BP_ThirdPersonCharacter.BP_ThirdPersonCharacter_C" (`KismetMathLibrary.Conv_VectorToTransform` _returnvalue_3) "AdjustIfPossibleButAlwaysSpawn" "OverrideRootScale" null null))
      (else
        (bind _returnvalue_4 (`self.GetP0Respawn`))
        (`|SpawnActorFromClass` "/Game/Blueprints/BP_ThirdPersonCharacter2.BP_ThirdPersonCharacter2_C" (`KismetMathLibrary.Conv_VectorToTransform` _returnvalue_4) "AdjustIfPossibleButAlwaysSpawn" "OverrideRootScale" null null)))))

(event `self.ResetProgress`
  (`KismetSystemLibrary.PrintString` "RESET")
  (bind _returnvalue (`GameplayStatics.CreateSaveGameObject` "/Game/Blueprints/BP_SaveGameInfo.BP_SaveGameInfo_C"))
  (bind _output_get (set `self.Save Game Instance` _returnvalue))
  (`|ExecutionSequence`
    (:`then_0`
      (set `/Game/Blueprints/BP_SaveGameInfo.L1AllCollectablesFound` false _output_get))
    (:`then_1`
      (set `/Game/Blueprints/BP_SaveGameInfo.L2AllCollectablesFound` false _output_get))
    (:`then_2`
      (set `/Game/Blueprints/BP_SaveGameInfo.L3AllCollectablesFound` false _output_get))
    (:`then_3`
      (set `/Game/Blueprints/BP_SaveGameInfo.L1CollectablesFound` 0 _output_get))
    (:`then_4`
      (set `/Game/Blueprints/BP_SaveGameInfo.L2CollectablesFound` 0 _output_get))
    (:`then_5`
      (set `/Game/Blueprints/BP_SaveGameInfo.L3CollectablesFound` 0 _output_get))
    (:`then_6`
      (`KismetArrayLibrary.Array_Clear` (`/Game/Blueprints/BP_SaveGameInfo.CollectablesFound` _output_get)))
    (:`then_7`
      (`AsyncActionHandleSaveGame.AsyncSaveGameToSlot` _output_get (`/Game/Blueprints/BP_SaveGameInfo.SaveSlotName` _output_get) (`/Game/Blueprints/BP_SaveGameInfo.UserIndex` _output_get)))))

(event `SwapControl`
  (bind _returnvalue (`GameMapsSettings.GetGameMapsSettings`))
  (if (`GameMapsSettings.GetSkipAssigningGamepadToPlayer1` _returnvalue)
    (`GameMapsSettings.SetSkipAssigningGamepadToPlayer1` _returnvalue false)
    (else
      (`GameMapsSettings.SetSkipAssigningGamepadToPlayer1` _returnvalue true))))

(event `self.SaveAddPlayer`
  (bind _returnvalue (`self.GetTwoPlayer`))
  (bind _asbp_game_instance (cast `/Game/Blueprints/BP_GameInstance` (`GameplayStatics.GetGameInstance`)))
  (set `/Game/Blueprints/BP_GameInstance.twoPlayersInst` _returnvalue _asbp_game_instance))

(fn `UserConstructionScript`)