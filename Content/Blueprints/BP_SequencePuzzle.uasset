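; Sequence puzzle actor that requires objects to be triggered in a set order.
; CheckCompletion compares the passed object to the entry at the current stage, advancing with a sound on a match.
; Completing the sequence marks the puzzle complete, increments each linked object's InteractsActive count and calls OnActivate on it.
; A wrong input resets the stage and deactivates and untoggles every sequence object.
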(fn `CheckCompletion`
  (params (NewParam :type "Interactable Object Reference"))
  (bind _objects (`self.Objects`))
  (bind _stage (`self.stage`))
  (if (== NewParam (`|GetArrayItem` _objects _stage))
    (`KismetSystemLibrary.PrintString` "correct sequence")
    (`GameplayStatics.PlaySound2D` "/Game/Audio/GameAudio/StatueCorrect.StatueCorrect" 1.0 1.0 0.0 null null)
    (`/Engine/EditorBlueprintResources/StandardMacros.IncrementInt` _stage
      (:`  `
        (if (== (`self.stage`) (`KismetArrayLibrary.Array_Length` (`self.Objects`)))
          (set `self.isComplete` true)
          (`KismetSystemLibrary.PrintString` "puzzle complete")
          (`GameplayStatics.PlaySound2D` "/Game/Audio/GameAudio/Puzzle_finsihed.Puzzle_finsihed" 1.0 1.0 0.0 null null)
          (for _array_element (`self.activatedObjectArray`)
            (bind _result (`/Engine/EditorBlueprintResources/StandardMacros.IncrementInt` (`Activatable.interactsActive` _array_element))
              (:`  `
                (set `Activatable.interactsActive` _result _array_element)
                (`Activatable.OnActivate` _array_element)))))))
    (else
      (`KismetSystemLibrary.PrintString` "wrong sequence")
      (`GameplayStatics.PlaySound2D` "/Game/Audio/GameAudio/incorrect.incorrect" 1.0 1.0 0.0 null null)
      (set `self.stage` 0)
      (for _array_element_2 _objects
        (`self.DeActivateLoop` _array_element_2)
        (set `Interactable.isToggled` false _array_element_2)))))

(fn `UserConstructionScript`)