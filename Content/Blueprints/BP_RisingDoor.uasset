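; BP_RisingDoor is a door whose cube rises by a set amount when activated with exactly the required number of active interacts.
; OnActivate computes the raised position and slides the cube there with a timed MoveComponentTo, guarded against retriggering while moving.
; StopActivate returns an activated door to the location saved at BeginPlay, without that guard.
; Debug prints and an unconnected lerp-based movement branch remain.
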(event `self.ReceiveTick`
  (params (DeltaSeconds :type "Float (single-precision)")))

(event `self.ReceiveBeginPlay`
  (set `self.oldHeight` (`SceneComponent.RelativeLocation` (`self.Cube`))))

(event `self.OnActivate`
  (bind _cube (`self.Cube`))
  (if (== (`self.interactsNeeded`) (`self.interactsActive`))
    (if (not (`self.isMoving`))
      (`KismetSystemLibrary.PrintString` "true")
      (`KismetMathLibrary.Vector_Set` (`self.newHeight`) (.x (`SceneComponent.RelativeLocation` (`self.Cube`))) (.y (`SceneComponent.RelativeLocation` (`self.Cube`))) (+ (.z (`SceneComponent.RelativeLocation` (`self.Cube`))) (`self.RaiseAmount`)))
      (set `self.isMoving` true)
      (`KismetSystemLibrary.MoveComponentTo` _cube (`self.newHeight`) (`SceneComponent.RelativeRotation` _cube) false false (`self.timeToRise`))
      (set `self.isMoving` false)
      (set `self.isActivated` true))
    (else
      (`KismetSystemLibrary.PrintString` "fakse"))))

(event `self.StopActivate`
  (bind _cube (`self.Cube`))
  (if (`self.isActivated`)
    (set `self.isMoving` true)
    (`KismetSystemLibrary.MoveComponentTo` _cube (`self.oldHeight`) (`SceneComponent.RelativeRotation` _cube) false false (`self.timeToRise`))
    (set `self.isMoving` false)
    (set `self.isActivated` false)))

(fn `UserConstructionScript`)