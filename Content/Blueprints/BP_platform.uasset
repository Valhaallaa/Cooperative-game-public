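; Platform actor that moves between OldHeight and NewHeight, with activation gated by InteractsActive equalling InteractsNeeded.
; OnActivate stores the current location and runs the lerp once, while Tick increments the alpha and applies the same lerp every frame, ungated and unclamped.
; StopActivate snaps back to OldHeight and clears IsActivated, though Tick keeps setting both.
; The RiseAmount-based NewHeight calculation is disconnected and never runs.
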(event `self.ReceiveTick`
  (params (DeltaSeconds :type "Float (single-precision)"))
  (bind _result (`/Engine/EditorBlueprintResources/StandardMacros.IncrementFloat` (`self.NewVar_0`))
    (:`  `
      (bind _output_get (set `self.NewVar_0` _result))
      (`self.K2_SetActorLocation` (`KismetMathLibrary.VLerp` (stale `self.OnActivate` _output_get) (`self.newHeight`) _output_get) :!label _label)
      (set `self.isActivated` true))))

(event `self.OnActivate`
  (if (== (`self.interactsNeeded`) (`self.interactsActive`))
    (`KismetSystemLibrary.PrintString` "true")
    (bind _output_get (set `self.oldHeight` (`self.K2_GetActorLocation`)))
    (goto _label)
    (else
      (`KismetSystemLibrary.PrintString` "fakse"))))

(event `self.StopActivate`
  (if (`self.isActivated`)
    (`self.K2_SetActorLocation` (`self.oldHeight`))
    (set `self.isActivated` false)))

(fn `UserConstructionScript`)