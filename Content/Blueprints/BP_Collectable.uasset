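; BP_Collectable is a spinning pickup that the player characters collect by touching it.
; Tick yaws the actor at a rate set by Speed, and Cube's overlap accepts either BP_ThirdPersonCharacter or BP_ThirdPersonCharacter2.
; On pickup it calls CollectCollectable, adds itself to CollectablesFound on BP_Gamemode's SaveGameInstance, then destroys itself.
; The two character branches duplicate the same logic, and the destroy only runs if the game mode cast succeeds.
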(event `self.ReceiveTick`
  (params (DeltaSeconds :type "Float (single-precision)"))
  (`self.K2_AddActorLocalRotation` (`KismetMathLibrary.MakeRotator` 0.0 0.0 (* DeltaSeconds (`self.Speed`)))))

(event `self.Cube.OnComponentBeginOverlap`
  (params (OverlappedComponent :type "PrimitiveComponent Object Reference") (OtherActor :type "Actor Object Reference") (OtherComp :type "PrimitiveComponent Object Reference") (OtherBodyIndex :type Integer) (bFromSweep :type Boolean) (SweepResult :type "HitResult Structure (by ref)"))
  (cast `/Game/Blueprints/BP_ThirdPersonCharacter` OtherActor
    (:`then`
      (`self.collect Collectable`)
      (bind _asbp_gamemode (cast `/Game/Blueprints/BP_Gamemode` (`GameplayStatics.GetGameMode`)))
      (`KismetArrayLibrary.Array_Add` (`/Game/Blueprints/BP_SaveGameInfo.CollectablesFound` (`/Game/Blueprints/BP_Gamemode.Save Game Instance` _asbp_gamemode)) self))
    (:`CastFailed`
      (cast `/Game/Blueprints/BP_ThirdPersonCharacter2` OtherActor)
      (`self.collect Collectable`)
      (bind _asbp_gamemode_2 (cast `/Game/Blueprints/BP_Gamemode` (`GameplayStatics.GetGameMode`)))
      (`KismetArrayLibrary.Array_Add` (`/Game/Blueprints/BP_SaveGameInfo.CollectablesFound` (`/Game/Blueprints/BP_Gamemode.Save Game Instance` _asbp_gamemode_2)) self)))
  (`self.K2_DestroyActor`))

(fn `UserConstructionScript`)