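; Door actor that opens by destroying itself when activated with the required number of active interacts.
; OnActivate calls DestroyActor only when InteractsActive equals InteractsNeeded.
; StopActivate teleport-free sets the location back to OldHeight and clears IsActivated if that flag is set.
; Nothing in this graph sets IsActivated true, stores OldHeight or updates the interact count.
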(event `self.OnActivate`
  (if (== (`self.interactsNeeded`) (`self.interactsActive`))
    (`self.K2_DestroyActor`)))

(event `self.StopActivate`
  (if (`self.isActivated`)
    (`self.K2_SetActorLocation` (`self.oldHeight`))
    (set `self.isActivated` false)))

(fn `UserConstructionScript`)