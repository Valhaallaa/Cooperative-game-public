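; Campfire checkpoint actor that lights up and sets new respawn points for two players.
; When either of the two third-person character classes overlaps the trigger, it fires once, marking itself reached, showing the fire and passing two cube markers' locations to BP_Gamemode as respawn positions.
; The overlap also enables the actor's input for player controller 0, and any end overlap disables it, though no input events are defined.
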(event `self.trigger.OnComponentBeginOverlap`
  (params (OverlappedComponent :type "PrimitiveComponent Object Reference") (OtherActor :type "Actor Object Reference") (OtherComp :type "PrimitiveComponent Object Reference") (OtherBodyIndex :type Integer) (bFromSweep :type Boolean) (SweepResult :type "HitResult Structure (by ref)"))
  (if (not (`self.CheckpointReached`))
    (cast `/Game/Blueprints/BP_ThirdPersonCharacter` OtherActor
      (:`then`
        _)
      (:`CastFailed`
        (cast `/Game/Blueprints/BP_ThirdPersonCharacter2` OtherActor)))
    (`self.EnableInput` (`GameplayStatics.GetPlayerController` 0))
    (`/Engine/EditorBlueprintResources/StandardMacros.DoOnce` false
      (:`Completed`
        (set `self.CheckpointReached` true)
        (`SceneComponent.SetVisibility` (`self.Fire`) true false)
        (bind _asbp_gamemode (cast `/Game/Blueprints/BP_Gamemode` (`GameplayStatics.GetGameMode`)))
        (`MyProjectGameMode.UpdateBothRespawn` _asbp_gamemode (`SceneComponent.K2_GetComponentLocation` (`self.Cube`)) (`SceneComponent.K2_GetComponentLocation` (`self.Cube1`)))))))

(event `self.trigger.OnComponentEndOverlap`
  (params (OverlappedComponent :type "PrimitiveComponent Object Reference") (OtherActor :type "Actor Object Reference") (OtherComp :type "PrimitiveComponent Object Reference") (OtherBodyIndex :type Integer))
  (`self.DisableInput` (`GameplayStatics.GetPlayerController` 0)))

(fn `UserConstructionScript`)