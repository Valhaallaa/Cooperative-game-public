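; Rotating platform actor that turns by a set yaw amount once enough interacts are active.
; OnActivate compares the active and needed interact counts, then sets a yaw-offset target and enables movement.
; Tick eases the actor toward it by lerping from its current rotation, using TimeToRotate as alpha, until they match.
; StopActivate instead uses MoveComponentTo with the mesh's reversed yaw offset over TimeToRotate and sets IsActivated.
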(event `self.ReceiveTick`
  (params (DeltaSeconds :type "Float (single-precision)"))
  (bind _returnvalue (`self.K2_GetActorRotation`))
  (if (`self.shouldMove`)
    (`self.K2_SetActorRotation` (`KismetMathLibrary.RLerp` _returnvalue (`self.rot`) (`self.timeToRotate`)))
    (if (== _returnvalue (stale `self.OnActivate` _output_get))
      (set `self.shouldMove` false))))

(event `self.OnActivate`
  (if (== (`self.interactsNeeded`) (`self.interactsActive`))
    (`KismetSystemLibrary.PrintString` "true")
    (bind _output_get (set `self.rot` (`KismetMathLibrary.MakeRotator` (.roll (`self.K2_GetActorRotation`)) (.pitch (`self.K2_GetActorRotation`)) (+ (.yaw (`self.K2_GetActorRotation`)) (`self.ZrotationAmount`)))))
    (set `self.shouldMove` true)
    (else
      (`KismetSystemLibrary.PrintString` "false"))))

(event `self.StopActivate`
  (`KismetSystemLibrary.MoveComponentTo` null (0.0 0.0 0.0) (`KismetMathLibrary.MakeRotator` (.roll (`SceneComponent.RelativeRotation` (`self.StaticMesh`))) (.pitch (`SceneComponent.RelativeRotation` (`self.StaticMesh`))) (- (.yaw (`SceneComponent.RelativeRotation` (`self.StaticMesh`))) (`self.ZrotationAmount`))) false false (`self.timeToRotate`))
  (set `self.isActivated` true))

(fn `UserConstructionScript`)