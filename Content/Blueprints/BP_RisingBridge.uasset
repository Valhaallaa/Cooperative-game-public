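; BP_RisingBridge is a bridge actor that rises when activated and returns when deactivated.
; OnActivate requires InteractsActive to equal InteractsNeeded, then saves the current location and instantly moves the actor up by RiseAmount, without sweep or interpolation.
; StopActivate restores the saved location if IsActivated is set.
; Debug prints remain in both activation branches, and nothing in this graph updates the interact counts.
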(event `self.OnActivate`
  (bind _returnvalue (`self.K2_GetActorLocation`))
  (bind _newheight (`self.newHeight`))
  (if (== (`self.interactsNeeded`) (`self.interactsActive`))
    (`KismetSystemLibrary.PrintString` "true")
    (set `self.oldHeight` _returnvalue)
    (`KismetMathLibrary.Vector_Set` _newheight (.x _returnvalue) (.y _returnvalue) (+ (.z _returnvalue) (`self.Rise Amount`)))
    (`KismetSystemLibrary.PrintString` "Hello")
    (`self.K2_SetActorLocation` _newheight)
    (set `self.isActivated` true)
    (else
      (`KismetSystemLibrary.PrintString` "fakse"))))

(event `self.StopActivate`
  (if (`self.isActivated`)
    (`self.K2_SetActorLocation` (`self.oldHeight`))
    (set `self.isActivated` false)))

(fn `UserConstructionScript`)