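; Trigger actor that releases a boulder when a Character overlaps its Cube component.
; The overlap enables physics simulation on the referenced Boulder's sphere and launches it with a fixed horizontal velocity-change impulse.
; It then teleports the ThingtoVisible actor to BlockLocation.
; A disconnected branch that would destroy Thingtodestroy before the impulse never runs.
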(event `self.ReceiveBeginPlay`)

(event `self.Cube.OnComponentBeginOverlap`
  (params (OverlappedComponent :type "PrimitiveComponent Object Reference") (OtherActor :type "Actor Object Reference") (OtherComp :type "PrimitiveComponent Object Reference") (OtherBodyIndex :type Integer) (bFromSweep :type Boolean) (SweepResult :type "HitResult Structure (by ref)"))
  (bind _boulder (`self.Boulder`))
  (cast `Character` OtherActor)
  (`PrimitiveComponent.SetSimulatePhysics` (`/Game/Blueprints/BP_Boulder.Sphere1` _boulder) true)
  (`PrimitiveComponent.AddImpulse` (`/Game/Blueprints/BP_Boulder.Sphere1` _boulder) (20.0 20.0 0.0) "None" true)
  (`self.K2_SetActorLocation` (`self.ThingtoVisible`) (`self.Block Location`) false true))

(fn `UserConstructionScript`)