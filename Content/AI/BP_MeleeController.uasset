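; BP_MeleeController is an AI controller for melee enemies that picks the nearer of two player-type characters as its target.
; It caches MyProjectCharacter actors on BeginPlay and starts BT_EnemyMelee on the first Tick.
; Later ticks, while either of the first two is within 1000 units, write the closer one to the Blackboard, plus a bool for whether it is still beyond melee distance.
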(event `self.ReceiveBeginPlay`
  (bind _outactors (`GameplayStatics.GetAllActorsOfClass` "/Script/MyProject.MyProjectCharacter"))
  (set `self.Out Actors` _outactors))

(event `self.ReceiveTick`
  (params (DeltaSeconds :type "Float (single-precision)"))
  (bind _returnvalue (`AIBlueprintHelperLibrary.GetBlackboard` null))
  (bind _out_actors (`self.Out Actors`))
  (bind _key_name (`self.Key Name`))
  (bind _returnvalue_2 (`KismetMathLibrary.Vector_Distance` (`self.K2_GetActorLocation` (`|GetArrayItem` _out_actors 1)) (`self.K2_GetActorLocation`)))
  (bind _returnvalue_3 (`KismetMathLibrary.Vector_Distance` (`self.K2_GetActorLocation` (`|GetArrayItem` _out_actors)) (`self.K2_GetActorLocation`)))
  (if (`self.setip`)
    (if (or (>= 1000.0 _returnvalue_3) (>= 1000.0 _returnvalue_2))
      (if (> _returnvalue_3 _returnvalue_2)
        (`BlackboardComponent.SetValueAsObject` _returnvalue _key_name (`|GetArrayItem` (`self.Out Actors`) 1))
        (else
          (`BlackboardComponent.SetValueAsObject` _returnvalue _key_name (`|GetArrayItem` (`self.Out Actors`)))))
      (`BlackboardComponent.SetValueAsBool` (`AIBlueprintHelperLibrary.GetBlackboard` null) (`self.Key Name_0`) (<= 130.0 (`KismetMathLibrary.Vector_Distance` (`BlackboardComponent.GetLocationFromEntry` (`AIBlueprintHelperLibrary.GetBlackboard` null) _key_name) (`self.K2_GetActorLocation`)))))
    (else
      (set `self.setip` true)
      (`self.RunBehaviorTree` "/Game/AI/BehaviourTrees/BT_EnemyMelee.BT_EnemyMelee"))))

(fn `UserConstructionScript`)