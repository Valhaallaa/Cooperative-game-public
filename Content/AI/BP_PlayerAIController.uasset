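; AI controller that runs BT_PlayerAI on its pawn, with a toggleable recall toward the player and jumping across nav links.
; It stores the player pawn in the blackboard on startup, and Tick sets the recall key while Recalling is on and the pawn is at least 200 units away.
; On a reachable nav link, it launches the character with velocity computed by math expressions toward the destination and plays a jump sound.
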(event EventBeginPlay
  (bind _returnvalue (AI|GetBlackboard 0))
  (Variables|Default|SetRecall false)
  (AI|RunBehaviorTree "/Game/AI/BehaviourTrees/BT_PlayerAI.BT_PlayerAI")
  (AI|Components|Blackboard|SetValueasObject _returnvalue (Variables|Default|GetPlayer) (Game|Player|GetPlayerPawn 0))
  (AI|Components|Blackboard|SetValueasBool _returnvalue (Variables|Default|GetRecallkey) (Variables|Default|GetRecall)))

(event EventTick
  (params (DeltaSeconds :type Float%20%28single-precision%29))
  (bind _returnvalue (AI|GetBlackboard 0))
  (if (Utilities|IsValid (AI|Components|Blackboard|GetValueasObject (AI|GetBlackboard 0) (Variables|Default|GetPlayer)))
    (if (Variables|Default|Getrecalling)
      (if (> 2e+02 (Math|Vector|Distance(Vector) (Transformation|GetActorLocation (Game|Player|GetPlayerPawn 0)) (Transformation|GetActorLocation (stale EventPossess PossessedPawn))))
        (Variables|Default|SetRecall false :!label _label)
        (else
          (Variables|Default|SetRecall true)))
      (else
        (goto _label)))
    (AI|Components|Blackboard|SetValueasBool _returnvalue (Variables|Default|GetRecallkey) (Variables|Default|GetRecall))
    (else
      (AI|Components|Blackboard|SetValueasObject _returnvalue (Variables|Default|GetPlayer) (Game|Player|GetPlayerPawn 0))
      (AI|Components|Blackboard|SetValueasBool _returnvalue (Variables|Default|GetRecallkey) (Variables|Default|GetRecall)))))

(event EventPossess
  (params (PossessedPawn :type Pawn%20Object%20Reference))
  (bind _returnvalue (AI|GetBlackboard 0))
  (Variables|Default|SetRecall false)
  (AI|RunBehaviorTree "/Game/AI/BehaviourTrees/BT_PlayerAI.BT_PlayerAI")
  (AI|Components|Blackboard|SetValueasObject _returnvalue (Variables|Default|GetPlayer) (Game|Player|GetPlayerPawn 0))
  (AI|Components|Blackboard|SetValueasBool _returnvalue (Variables|Default|GetRecallkey) (Variables|Default|GetRecall)))

(event EventNavLinkReachable
  (params (Destination :type Vector :default "0, 0, 0"))
  (bind (_x _y _z) (Math|Vector|BreakVector Destination))
  (bind _ascharacter (Utilities|Casting|CastToCharacter (stale EventPossess PossessedPawn)))
  (Character|LaunchCharacter _ascharacter (Math|Vector|MakeVector (|((DestinationX-startx)/{A153A4B2-4522-C183-1F14-BC9B336133A9}) _x (.X (Math|Vector|BreakVector (Transformation|GetActorLocation (stale EventPossess PossessedPawn))))) (|((DestinationY-starty)/{A153A4B2-4522-C183-1F14-BC9B336133A9}) _y (.Y (Math|Vector|BreakVector (Transformation|GetActorLocation (stale EventPossess PossessedPawn))))) (|((DestinationH-(StartH-(((Power({A153A4B2-4522-C183-1F14-BC9B336133A9},2))*0.500000)*{0C2F1222-4802-4E00-477A-848EA7B06705})))/{A153A4B2-4522-C183-1F14-BC9B336133A9}) _z (.Z (Math|Vector|BreakVector (Transformation|GetActorLocation (stale EventPossess PossessedPawn)))))) true true)
  (Audio|PlaySound2D "/Game/Audio/GameAudio/FoleyAudio/Jump.Jump" 1.0 1.0 0.0 0 0))

(fn ConstructionScript)

(fn SetRecall
  (if (Variables|Default|Getrecalling)
    (Variables|Default|Setrecalling false)
    (else
      (Variables|Default|Setrecalling true)))
  (AI|Components|Blackboard|SetValueasBool (AI|GetBlackboard 0) (Variables|Default|GetRecallkey) (Variables|Default|GetRecall)))